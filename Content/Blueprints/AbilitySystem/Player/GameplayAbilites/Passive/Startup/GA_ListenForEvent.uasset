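; Passive gameplay ability that listens for Attributes gameplay events and turns them into attribute changes on its owner.
; On activation it waits continuously for events under the Attributes tag, including child tags.
; Each event builds a GEEventBasedEffectClass spec and applies it to self.
; SetByCaller magnitudes come from EventTags: the exact match receives the event's magnitude, and all others get zero to avoid missing-magnitude errors.
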(event `self.K2_ActivateAbility`
  (bind _returnvalue (`self.GetAbilitySystemComponentFromActorInfo`))
  (bind (_asynctaskproxy _payload) (`AbilityTask_WaitGameplayEvent.WaitGameplayEvent` (struct :`TagName` "Attributes") null false false) ; OnlyTriggerOnce为False 任务就会一直监听事件
    (:`EventReceived`
      (bind (_eventtag _instigator _target _optionalobject _optionalobject2 _contexthandle _instigatortags _targettags _eventmagnitude) (break `GameplayEventData` _payload))
      (set `self.EventTag` _eventtag)
      (set `self.EventMagnitude` _eventmagnitude)
      (set `self.EffectSpecHandle` (`AbilitySystemComponent.MakeOutgoingSpec` _returnvalue (`self.GE_EventBasedEffectClass`) 1.0 (`AbilitySystemComponent.MakeEffectContext` _returnvalue)))
      (for _array_element (`self.EventTags`)
        (if (`BlueprintGameplayTagLibrary.MatchesTag` _array_element (`self.EventTag`) true)
          (`AbilitySystemBlueprintLibrary.AssignTagSetByCallerMagnitude` (`self.EffectSpecHandle`) (`self.EventTag`) (`self.EventMagnitude`))
          (else
            (`AbilitySystemBlueprintLibrary.AssignTagSetByCallerMagnitude` (`self.EffectSpecHandle`) _array_element))))
      (`AbilitySystemComponent.BP_ApplyGameplayEffectSpecToSelf` (`self.GetAbilitySystemComponentFromActorInfo`) (`self.EffectSpecHandle`)))))