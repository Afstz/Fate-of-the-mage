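; Player gameplay ability for a held lightning chain that shocks the target under the mouse and arcs to additional targets.
; A montage event locks movement, adds ShockLoop cues to the targets and starts a looping damage timer.
; Each tick pays the cost and applies damage effects on authority if the first target implements CombatInterface.
; Input release, failed cost or first-target death ends it with cleanup and cooldown; other deaths only drop their chain.
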(event `DamageEvent`
  ;[1 0.573 0.4931] Caused Damage
  (bind _returnvalue (`self.K2_CommitAbilityCost` false))
  (if _returnvalue
    (if (`self.FirstTargetImplementCombatInteface`)
      (`self.ApplyDamage`))
    (else
      (`self.ClearTimerHandleAndEndAbility`))))

(event `self.K2_ActivateAbility`
  (if (`KismetSystemLibrary.DoesImplementInterface` (`self.GetAvatarActorFromActorInfo`) "/Script/Mage.CombatInterface")
    ;[1 1 1] 保存HitResult变量
    (bind (_asynctaskproxy _data) (`TargetDataUnderMouse.CreateTargetDataUnderMouse`)
      (:`MouseTargetValidData`
        (`self.StoreMouseHitResult` (`AbilitySystemBlueprintLibrary.GetHitResultFromTargetData` _data))
        (`self.StoreOwnerVariables`)
        (`|ExecutionSequence`
          (:`then_0`
            (message `CombatInterface.UpdateFacingTarget` (`self.GetAvatarActorFromActorInfo`) (`self.MouseHitLocation`))
            (`self.K2_ExecuteGameplayCue` (struct :`TagName` "GameplayCue.ShockBurst")) ; 播放释放闪电链的音效
            (`AbilityTask_PlayMontageAndWait.CreatePlayMontageAndWaitProxy` "None" (`self.ShockMontage`) 1.0 "None" false
              (:`then`
                (`AbilityTask_WaitGameplayEvent.WaitGameplayEvent` (struct :`TagName` "Event.Montage.LightningChain") null true
                  (:`EventReceived`
                    (`self.InShockLoop`)
                    (`self.SpawnLightningChain`)
                    ;[1 0.573 0.4931] Caused Damage
                    (bind _returnvalue (`KismetSystemLibrary.K2_SetTimerDelegate` (delegate `DamageEvent`) (`self.DamageDeltaTime`) true))
                    (set `self.DamageTimerHandle` _returnvalue))))))
          (:`then_1`
            ;[1 1 1] 松开按键结束技能
            (`AbilityTask_WaitInputRelease.WaitInputRelease` false
              (:`OnRelease`
                (`self.ClearTimerHandleAndEndAbility`)))))))
    (else
      (`self.K2_EndAbility`))))

(event `self.FirstTargetDied`
  (params (FirstTarget :type "Actor Object Reference"))
  ;[1 1 1] 首个目标死亡，结束技能
  (`GameplayCueFunctionLibrary.RemoveGameplayCueOnActor` FirstTarget (struct :`TagName` "GameplayCue.ShockLoop") (`self.FirstTargetCueParams`))
  (`self.ClearTimerHandleAndEndAbility`))

(event `self.AdditionalTargetDied`
  (params (AdditionalTarget :type "Actor Object Reference"))
  ;[1 1 1] 额外目标死亡,清除对应闪电链特效
  (`self.RemoveAdditionalShockLoopCue` AdditionalTarget)
  (`KismetArrayLibrary.Array_RemoveItem` (`self.AdditionalTargets`) AdditionalTarget))

(fn `ApplyDamage`
  (`self.ApplyDamageForSingle` (`self.MouseHitActor`))
  (for _array_element (`self.AdditionalTargets`)
    (`self.ApplyDamageForSingle` _array_element)))

(fn `ApplyDamageForSingle`
  (params (TargetActor :type "Actor Object Reference"))
  (locals (Target :type "Actor Object Reference"))
  (`self.K2_HasAuthority` ; 伤害计算在服务器上执行
    (:`True`
      (`MageAbilitySystemLibrary.ApplyDamageEffect` (`self.MakeDamageEffectParamsFromClassDefaults` TargetActor)))))

(fn `ClearTimerHandleAndEndAbility`
  (`KismetSystemLibrary.K2_ClearAndInvalidateTimerHandle` (`self.DamageTimerHandle`))
  (`self.PrepareToEndAbility`)
  (`self.K2_CommitAbilityCooldown` false)
  (`self.ClearVariablesAndDelegates`)
  (`self.K2_EndAbility`))

(fn `ClearVariablesAndDelegates`
  (`self.ClearDelegate` (`self.CueTarget`))
  (for _array_element (`self.AdditionalTargets`)
    (`self.ClearDelegate` _array_element)
    (`KismetArrayLibrary.Array_Clear` (`self.AdditionalTargets`))
    (`BlueprintMapLibrary.Map_Clear` (`self.AdditionalTargetsToCueParams`))))

(fn `InShockLoop`
  (message `CombatInterface.SetInShockLoop` (`self.OwnerCharacter`) true)
  (`CharacterMovementComponent.DisableMovement` (`Character.CharacterMovement` (`self.OwnerCharacter`))))

(fn `PrepareToEndAbility`
  (message `CombatInterface.SetInShockLoop` (`self.OwnerCharacter`) false)
  (`CharacterMovementComponent.SetMovementMode` (`Character.CharacterMovement` (`self.OwnerCharacter`)) "MOVE_Walking" 0)
  (`GameplayCueFunctionLibrary.RemoveGameplayCueOnActor` (`self.CueTarget`) (struct :`TagName` "GameplayCue.ShockLoop") (`self.FirstTargetCueParams`))
  (message `CombatInterface.SetBeingShocked` (`self.CueTarget`) false)
  (for _array_element (`self.AdditionalTargets`)
    (`self.RemoveAdditionalShockLoopCue` _array_element)
    (message `CombatInterface.SetBeingShocked` _array_element false)))

(fn `RemoveAdditionalShockLoopCue`
  (params (AdditionalActor :type "Actor Object Reference"))
  (locals (TargetActor :type "Actor Object Reference"))
  (bind _output_get (set `local.TargetActor` AdditionalActor))
  (bind (_value _returnvalue) (`BlueprintMapLibrary.Map_Find` (`self.AdditionalTargetsToCueParams`) _output_get))
  (if _returnvalue
    (`GameplayCueFunctionLibrary.RemoveGameplayCueOnActor` (`local.TargetActor`) (struct :`TagName` "GameplayCue.ShockLoop") _value)))

(fn `SpawnAdditionalLightningChain`
  (params (AdditionalTarget :type "Actor Object Reference (by ref)"))
  (locals (TargetActor :type "Actor Object Reference"))
  (bind _targetactor (`local.TargetActor`))
  (bind _returnvalue (`AbilitySystemBlueprintLibrary.MakeGameplayCueParameters` 0.0 0.0 (struct) (struct) (struct) (struct) (struct) (`Actor.K2_GetActorLocation` _targetactor) (0.0 0.0 0.0) null null _targetactor null 1 1 (`Actor.RootComponent` (`self.MouseHitActor`))))
  (set `local.TargetActor` AdditionalTarget)
  (`BlueprintMapLibrary.Map_Add` (`self.AdditionalTargetsToCueParams`) (`local.TargetActor`) _returnvalue)
  (`GameplayCueFunctionLibrary.AddGameplayCueOnActor` (`local.TargetActor`) (struct :`TagName` "GameplayCue.ShockLoop") _returnvalue))

(fn `SpawnLightningChain`
  (`self.TraceFirstTarget` (`self.MouseHitLocation`))
  (bind _returnvalue (message `CombatInterface.GetWeaponMesh` (`self.GetAvatarActorFromActorInfo`)))
  (set `self.FirstTargetCueParams` (`AbilitySystemBlueprintLibrary.MakeGameplayCueParameters` 0.0 0.0 (struct) (struct) (struct) (struct) (struct) (`self.MouseHitLocation`) (0.0 0.0 0.0) null null (`self.MouseHitActor`) null 1 1 _returnvalue))
  ;[1 1 1] 击中的是否是敌人,根据对应的目标生成Cue
  (bind _output_get (set `self.FirstTargetImplementCombatInteface` (`KismetSystemLibrary.DoesImplementInterface` (`self.MouseHitActor`) "/Script/Mage.CombatInterface")))
  (if _output_get
    (set `self.CueTarget` (`self.MouseHitActor`))
    (else
      (set `self.CueTarget` (`self.GetAvatarActorFromActorInfo`))))
  (`GameplayCueFunctionLibrary.AddGameplayCueOnActor` (`self.CueTarget`) (struct :`TagName` "GameplayCue.ShockLoop") (`self.FirstTargetCueParams`))
  (if (`self.FirstTargetImplementCombatInteface`)
    (message `CombatInterface.SetBeingShocked` (`self.CueTarget`) true)
    ;[1 1 1] Additional Targets
    (bind _outadditionaltargets (`self.StoreAdditionalTargets`))
    (bind _output_get_2 (set `self.AdditionalTargets` _outadditionaltargets))
    (for _array_element _output_get_2
      (`self.SpawnAdditionalLightningChain` _array_element)
      (message `CombatInterface.SetBeingShocked` _array_element true))))