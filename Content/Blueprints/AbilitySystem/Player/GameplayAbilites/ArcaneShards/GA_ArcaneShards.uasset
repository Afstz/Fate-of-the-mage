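; Player gameplay ability that casts a series of damaging arcane shards around a mouse-targeted ground point.
; A magic circle shows until input release, then a point collection generates level-scaled ground points and a motion-warped cast montage plays.
; A montage gameplay event commits cost and starts a looping timer, spawning one shard cue per point with radial damage to non-friendly characters.
; Ending the ability clears the timer and points and commits cooldown.
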(event `self.K2_ActivateAbility`
  (bind _returnvalue (`self.K2_CheckAbilityCost`))
  (if _returnvalue
    (`|ExecutionSequence`
      (:`then_0`
        ;[0.3783 0.3917 1] Show Magic Circle
        (`self.IsLocallyControlled`
          (:`True`
            (message `PlayerInterface.ShowMagicCircle` (`self.GetAvatarActorFromActorInfo`) null))))
      (:`then_1`
        (`AbilityTask_WaitInputRelease.WaitInputRelease` false
          (:`OnRelease`
            (message `PlayerInterface.HideMagicCircle` (`self.GetAvatarActorFromActorInfo`))
            ;[1 0.4906 0.4107] Get Mouse Hit Location
            (bind (_asynctaskproxy _data) (`TargetDataUnderMouse.CreateTargetDataUnderMouse`)
              (:`MouseTargetValidData`
                (set `self.MouseHitLocation` (`.ImpactPoint` (`GameplayStatics.BreakHitResult` (`AbilitySystemBlueprintLibrary.GetHitResultFromTargetData` _data))))
                (`|ExecutionSequence`
                  (:`then_0`
                    ;[1 0.05018 0.02034] Spawn Point Collection
                    (bind _returnvalue_2 (`|SpawnActorFromClass` "/Game/Blueprints/AbilitySystem/Player/GameplayAbilites/ArcaneShards/BP_PointCollection.BP_PointCollection_C" (`KismetMathLibrary.MakeTransform` (`self.MouseHitLocation`)) "Undefined" "MultiplyWithRoot" null null))
                    (set `self.PointCollection` _returnvalue_2)
                    (set `self.ValidPoints` (`PointCollection.GetGroundPoints` (`self.PointCollection`) (`self.MouseHitLocation`) (`self.GetCurrentShardsNum` (`self.GetAbilityLevel`)) (`KismetMathLibrary.RandomFloatInRange` 0.0 360.0))))
                  (:`then_1`
                    ;[1 0.8085 0.234] Update Motion Warping Target
                    (message `CombatInterface.UpdateFacingTarget` (`self.GetAvatarActorFromActorInfo`) (`self.MouseHitLocation`)))
                  (:`then_2`
                    (`AbilityTask_PlayMontageAndWait.CreatePlayMontageAndWaitProxy` "None" "/Game/Assets/Characters/EgyptGirl/Animations/Abilities/AM_Cast_ArcaneShards.AM_Cast_ArcaneShards" 1.0 "None" false
                      (:`then`
                        (`AbilityTask_WaitGameplayEvent.WaitGameplayEvent` (struct :`TagName` "Event.Montage.ArcaneShards") null true
                          (:`EventReceived`
                            ;[0 1 0.2804] Set Timer Event And Spawn First Shards
                            (bind _returnvalue_3 (`KismetSystemLibrary.K2_SetTimerDelegate` (delegate `SpawnShards`) (`self.SpawnShardDeltaTime`) true))
                            (set `self.SpawnShardsTimer` _returnvalue_3)
                            (`self.SpawnShards`)
                            (`self.K2_CommitAbilityCost` false)))))))))))))))

(event `SpawnShards`
  (if (< (`self.LoopCount`) (`self.GetCurrentShardsNum` (`self.GetAbilityLevel`)))
    (`self.StoreShardSpawnLocation`)
    (`self.ExecuteArcaneShardCue`)
    (`self.ApplyRadialDamageToPlayers`)
    (`/Engine/EditorBlueprintResources/StandardMacros.IncrementInt` (`self.LoopCount`))
    (else
      (`self.K2_HasAuthority`
        (:`True`
          (`self.K2_EndAbility`))))))

(event `self.K2_OnEndAbility`
  (params (bWasCancelled :type Boolean))
  (`KismetSystemLibrary.K2_ClearAndInvalidateTimerHandle` (`self.SpawnShardsTimer`))
  (set `self.LoopCount` 0)
  (bind _pointcollection (`self.PointCollection`)
    (:`then`
      (`Actor.K2_DestroyActor` _pointcollection))
    (:`else`
      _))
  (`self.K2_CommitAbilityCooldown` false))

(fn `ApplyRadialDamageToPlayers`
  (bind _returnvalue (`self.GetAvatarActorFromActorInfo`))
  (bind _outoverlappingactors (`MageAbilitySystemLibrary.GetAlivePlayerInSphereRadius` _returnvalue (`|MakeArray` _returnvalue) (`self.RadialDamageOuterRadius`) (`self.ShardSpawnLocation`))) ; 找到范围内所有的角色
  (bind _output_get (set `self.OverlappingPlayers` _outoverlappingactors))
  (for _array_element _output_get
    (if (`MageAbilitySystemLibrary.IsNotFriend` (`self.GetAvatarActorFromActorInfo`) _array_element)
      (`MageAbilitySystemLibrary.ApplyDamageEffect` (`self.MakeDamageEffectParamsFromClassDefaults` _array_element (`self.ShardSpawnLocation`) true 35.0)))))

(fn `ExecuteArcaneShardCue`
  (`GameplayCueFunctionLibrary.ExecuteGameplayCueOnActor` (`self.GetAvatarActorFromActorInfo`) (struct :`TagName` "GameplayCue.ArcaneShards") (`AbilitySystemBlueprintLibrary.MakeGameplayCueParameters` 0.0 0.0 (struct) (struct) (struct) (struct) (struct) (`self.ShardSpawnLocation`))))

(fn `StoreShardSpawnLocation`
  (set `self.ShardSpawnLocation` (`SceneComponent.K2_GetComponentLocation` (`|GetArrayItem` (`self.ValidPoints`) (`self.LoopCount`)))))