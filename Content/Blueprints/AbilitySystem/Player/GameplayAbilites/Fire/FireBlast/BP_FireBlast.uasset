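; Fireball actor for the FireBlast ability that flies outward, boomerangs back to its owner and explodes near them.
; On BeginPlay, the server runs an outgoing timeline to a point ahead, then a return timeline tracking the owner's current location.
; Within explode distance, it applies radial GAS damage to living non-friendly players in range, then destroys itself.
; Knockback and death impulse point away from the blast, with pitch forced to 45 degrees.
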(event `self.StartFireBlastTimeline`
  (`/Engine/EditorBlueprintResources/ActorMacros.Switch Has Authority`
    (:`Authority`
      ;[0.3517 0.4997 1] 存储起始点和终点
      (set `self.OriginLocation` (`self.K2_GetActorLocation`))
      (set `self.DestinationLocation` (+ (`self.OriginLocation`) (* (`self.GetActorForwardVector`) (`self.FlightingDistance`))))
      ;[1 0.6235 0.6036] OutgoingTimeline
      (bind (_direction _time) (`Timeline|OutgoingTimeline`) ; 火球向外Timeline
        (:`Update`
          (`self.K2_SetActorLocation` (`KismetMathLibrary.VLerp` (`self.OriginLocation`) (`self.DestinationLocation`) _time)) ; 更新火球的位置
        )
        (:`Finished`
          ;[0.3588 1 0.3152] ReturnTimeline
          (bind (_direction_2 _timeline) (`Timeline|ReturnTimeline`) ; 火球返回Timeline
            (:`Update`
              (`self.K2_SetActorLocation` (`KismetMathLibrary.VLerp` (`self.DestinationLocation`) (`self.K2_GetActorLocation` (`self.GetOwner`)) _timeline)) ; 更新火球的位置
              (if (`self.IsWithinExplodeDistance`)
                ;[1 0.09322 0.08327] Explode
                (`|ExecutionSequence`
                  (:`then_0`
                    (bind _outoverlappingactors (`MageAbilitySystemLibrary.GetAlivePlayerInSphereRadius` self (`|MakeArray` (`self.GetOwner`)) (`self.RadialDamageOuterRadius`) (`self.K2_GetActorLocation`))) ; 获取爆炸范围内的角色
                    (set `self.OverlappingPlayers` _outoverlappingactors))
                  (:`then_1`
                    (`MageAbilitySystemLibrary.SetRadialDamageEffectParams` (`self.DamageEffectParams`) true (`self.K2_GetActorLocation`) (`self.RadialDamageInnerRadius`) (`self.RadialDamageOuterRadius`))
                    (for _array_element (`self.OverlappingPlayers`)
                      (if (`MageAbilitySystemLibrary.IsNotFriend` (`self.GetOwner`) _array_element)
                        ;;[0.8757 1 0.4692] Apply Damage
                        (`MageAbilitySystemLibrary.SetEffectParamsTargetASC` (`self.DamageEffectParams`) (`AbilitySystemBlueprintLibrary.GetAbilitySystemComponent` _array_element))
                        (set `self.ForceDirection` (- (`self.K2_GetActorLocation` _array_element) (`self.K2_GetActorLocation`)))
                        (`MageAbilitySystemLibrary.SetKnockbackForceDirection` (`self.DamageEffectParams`) (`self.OverrideForceDirectionPitch`) 400.0)
                        (`MageAbilitySystemLibrary.SetDeathImpulseDirections` (`self.DamageEffectParams`) (`self.OverrideForceDirectionPitch`) 20000.0)
                        (`MageAbilitySystemLibrary.ApplyDamageEffect` (`self.DamageEffectParams`))))
                    (`self.K2_DestroyActor`)))))))))))

(event `self.ReceiveBeginPlay`
  (`self.StartFireBlastTimeline`))

(fn `IsWithinExplodeDistance`
  (returns (ReturnValue :type Boolean))
  (return (<= (`KismetMathLibrary.VSize` (- (`self.K2_GetActorLocation`) (`self.K2_GetActorLocation` (`self.GetOwner`)))) (`self.ExplodeDistance`))))

(fn `OverrideForceDirectionPitch`
  (returns (ReturnValue :type "Vector Structure"))
  (bind (_returnvalue_roll _returnvalue_pitch _returnvalue_yaw) (`KismetMathLibrary.BreakRotator` (`KismetMathLibrary.MakeRotFromX` (`self.ForceDirection`))))
  (return (`KismetMathLibrary.GetForwardVector` (`KismetMathLibrary.MakeRotator` _returnvalue_roll 45.0 _returnvalue_yaw))))

(fn `UserConstructionScript`)