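; Player Fire Ball gameplay ability that casts a projectile using the location under the mouse.
; On activation it commits, plays the cast montage, and gets the mouse hit location through a target data task.
; It turns the caster toward that point via CombatInterface, then waits for the montage's gameplay event to call SpawnProjectile with it.
; The ability ends when the montage completes, is interrupted or is cancelled.
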(event `self.K2_ActivateAbility`
  (`self.K2_CommitAbility`)
  (`AbilityTask_PlayMontageAndWait.CreatePlayMontageAndWaitProxy` "None" "/Game/Assets/Characters/EgyptGirl/Animations/Abilities/AM_Cast_FireBall.AM_Cast_FireBall" 1.0 "None" false
    (:`then`
      (bind (_asynctaskproxy _data) (`TargetDataUnderMouse.CreateTargetDataUnderMouse`)
        (:`MouseTargetValidData`
          (set `self.SpawnLocation` (`.Location` (`GameplayStatics.BreakHitResult` (`AbilitySystemBlueprintLibrary.GetHitResultFromTargetData` _data))))
          (bind _ascombat_interface (cast `CombatInterface` (`self.GetAvatarActorFromActorInfo`)))
          (`CombatInterface.UpdateFacingTarget` _ascombat_interface (`self.SpawnLocation`))
          (`AbilityTask_WaitGameplayEvent.WaitGameplayEvent` (struct :`TagName` "Event.Montage.FireBall") null
            (:`EventReceived`
              (`self.SpawnProjectile` (`self.SpawnLocation`)))))))
    (:`OnCompleted`
      (`self.K2_EndAbility` :!label _label))
    (:`OnInterrupted`
      (goto _label))
    (:`OnCancelled`
      (goto _label))))