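; Player fireball Gameplay Ability that launches homing projectiles toward the target under the mouse.
; On activation it commits and starts the cast montage, then takes mouse target data and turns the avatar toward the hit location through CombatInterface.
; A montage gameplay event times SpawnProjectiles, which receives the location, hit actor as homing target and an upward pitch override.
; The ability ends when the montage completes, blends out or is interrupted or cancelled.
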(event `self.K2_ActivateAbility`
  (`self.K2_CommitAbility`)
  (`AbilityTask_PlayMontageAndWait.CreatePlayMontageAndWaitProxy` "None" "/Game/Assets/Characters/EgyptGirl/Animations/Abilities/AM_Cast_FireBall.AM_Cast_FireBall" 1.0 "None" false
    (:`then`
      (bind (_asynctaskproxy _data) (`TargetDataUnderMouse.CreateTargetDataUnderMouse`)
        (:`MouseTargetValidData`
          (bind (_bblockinghit _binitialoverlap _time _distance _location _impactpoint _normal _impactnormal _physmat _hitactor) (`GameplayStatics.BreakHitResult` (`AbilitySystemBlueprintLibrary.GetHitResultFromTargetData` _data)))
          (set `self.TargetLocation` _location)
          (set `self.HomingTarget` _hitactor)
          (bind _ascombat_interface (cast `CombatInterface` (`self.GetAvatarActorFromActorInfo`)))
          (`CombatInterface.UpdateFacingTarget` _ascombat_interface (`self.TargetLocation`))
          (`AbilityTask_WaitGameplayEvent.WaitGameplayEvent` (struct :`TagName` "Event.Montage.FireBall") null true
            (:`EventReceived`
              (`self.SpawnProjectiles` (`self.TargetLocation`) true 35.0 (`self.HomingTarget`)))))))
    (:`OnCompleted`
      (`self.K2_EndAbility` :!label _label))
    (:`OnBlendOut`
      (goto _label))
    (:`OnInterrupted`
      (goto _label))
    (:`OnCancelled`
      (goto _label))))