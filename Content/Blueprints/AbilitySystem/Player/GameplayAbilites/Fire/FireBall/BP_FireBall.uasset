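; Fireball projectile actor for the player's fire ability.
; On BeginPlay it calls DelayEnableCollision to handle collision activation.
; Each tick it compares its current location with the previous frame's and destroys itself when the distance moved is at or below a threshold, removing stalled fireballs.
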(event `self.ReceiveBeginPlay`
  (`self.DelayEnableCollision`))

(event `self.ReceiveTick`
  (params (DeltaSeconds :type "Float (single-precision)"))
  (set `self.LastFrameLocaiton` (`self.CurrentFrameLocation`))
  (set `self.CurrentFrameLocation` (`self.K2_GetActorLocation`))
  (if (<= (`KismetMathLibrary.VSize` (- (`self.CurrentFrameLocation`) (`self.LastFrameLocaiton`))) (`self.ClosetThreshold`))
    (`self.K2_DestroyActor`)))

(fn `UserConstructionScript`)