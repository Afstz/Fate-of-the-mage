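; GA_Attack is a melee attack Gameplay Ability that turns the avatar toward its facing target through CombatInterface and plays a random tagged montage.
; The montage's gameplay event triggers a small sphere query at that montage's socket location for living players.
; Each non-friendly hit receives damage.
; The ability ends when the montage completes, is interrupted or cancelled, or when no montages are available.
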(event `self.K2_ActivateAbility`
  (bind _returnvalue (`self.GetAvatarActorFromActorInfo`))
  (bind _returnvalue_2 (`self.GetAvatarActorFromActorInfo`))
  (bind _attacktaggedmontage (`self.AttackTaggedMontage`))
  (bind _returnvalue_3 (message `EnemyInterface.GetFacingTarget` _returnvalue))
  (bind _ascombat_interface (cast `CombatInterface` _returnvalue))
  (`CombatInterface.UpdateFacingTarget` _ascombat_interface (`Actor.K2_GetActorLocation` _returnvalue_3)) ; 更新要面向的目标
  (bind _returnvalue_4 (message `EnemyInterface.GetTaggedMontage` (`self.GetAvatarActorFromActorInfo`))) ; 获取设置的蒙太奇结构体并随机抽取一个
  (bind _returnvalue_5 (`KismetArrayLibrary.Array_Length` _returnvalue_4))
  (if (> _returnvalue_5 0)
    (bind _output_get (set `self.AttackTaggedMontage` (`|GetArrayItem` _returnvalue_4 (`KismetMathLibrary.RandomIntegerInRange` 0 (- _returnvalue_5 1)))))
    (`AbilityTask_PlayMontageAndWait.CreatePlayMontageAndWaitProxy` "None" (`.CombatMontage` (break `TaggedMontage` _output_get))
      (:`then`
        (`AbilityTask_WaitGameplayEvent.WaitGameplayEvent` (`.MontageEventTag` (break `TaggedMontage` _attacktaggedmontage)) null ; 接收指定标签事件
          (:`EventReceived`
            (bind _returnvalue_6 (message `EnemyInterface.GetSocketLocationByTaggedMontage` _returnvalue_2 _attacktaggedmontage)) ; 通过结构体获取插槽位置
            (bind _outoverlappingactors (`MageAbilitySystemLibrary.GetAlivePlayerInSphereRadius` _returnvalue_2 (`|MakeArray` _returnvalue_2) 40.0 _returnvalue_6)) ; 查找攻击范围内的击中的角色
            (for _array_element _outoverlappingactors
              (if (`MageAbilitySystemLibrary.IsNotFriend` (`self.GetAvatarActorFromActorInfo`) _array_element)
                (`self.CauseDamage` _array_element))))))
      (:`OnCompleted`
        (`self.K2_EndAbility` :!label _label))
      (:`OnInterrupted`
        (goto _label))
      (:`OnCancelled`
        (goto _label)))
    (else
      (`self.K2_EndAbility`))))