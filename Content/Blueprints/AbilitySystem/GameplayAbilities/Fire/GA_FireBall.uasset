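; GA_FireBall is a gameplay ability that casts a fireball toward the point under the mouse.
; On activation it plays the cast montage, gets the cursor hit location through the TargetDtatUnderMouse task, and turns the avatar toward it via CombatInterface.
; It then waits for the montage's Event.Montage.FireBall gameplay event, spawns the projectile at that target location, and ends shortly after.
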(event `self.K2_ActivateAbility`
  (`AbilityTask_PlayMontageAndWait.CreatePlayMontageAndWaitProxy` "None" "/Game/Assets/Characters/EgyptGirl/Animations/Abilities/AM_Cast_FireBall.AM_Cast_FireBall"
    (:`then`
      (bind (_asynctaskproxy _data) (`TargetDataUnderMouse.CreateTargetDtatUnderMouse`)
        (:`MouseTargetValidData`
          (set `self.SpawnLocation` (`.Location` (`GameplayStatics.BreakHitResult` (`AbilitySystemBlueprintLibrary.GetHitResultFromTargetData` _data))))
          (bind _ascombat_interface (cast `CombatInterface` (`self.GetAvatarActorFromActorInfo`)))
          (`CombatInterface.FacingTarget` _ascombat_interface (`self.SpawnLocation`))
          (`AbilityTask_WaitGameplayEvent.WaitGameplayEvent` (struct :`TagName` "Event.Montage.FireBall") null
            (:`EventReceived`
              (`self.SpawnProjectile` (`self.SpawnLocation`))
              (`KismetSystemLibrary.Delay` 0.2)
              (`self.K2_EndAbility`))))))))