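; Shaman enemy summon ability that spawns random minions at shuffled spawn locations around the battlefield.
; It updates the avatar's facing target, plays the summon montage and waits for its gameplay event.
; A delayed loop then spawns a Niagara effect and a minion with a default controller at each point, facing outward from the summoner.
; Each spawn raises the summoner's minion count, and each minion's destruction lowers it.
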(event `self.K2_ActivateAbility`
  (bind _returnvalue (`self.GetAvatarActorFromActorInfo`))
  (bind _output (`|GetArrayItem` (`self.SpawnLocations`) (`self.SpawnIndex`)))
  (bind _returnvalue_2 (+ _output (0.0 0.0 50.0)))
  (bind _returnvalue_3 (message `EnemyInterface.GetFacingTarget` _returnvalue))
  (message `CombatInterface.UpdateFacingTarget` _returnvalue (`Actor.K2_GetActorLocation` _returnvalue_3))
  (`AbilityTask_PlayMontageAndWait.CreatePlayMontageAndWaitProxy` "None" "/Game/Assets/Enemies/Shaman/Animations/AM_Shaman_Summon.AM_Shaman_Summon"
    (:`then`
      (`AbilityTask_WaitGameplayEvent.WaitGameplayEvent` (struct :`TagName` "Montage.Attack.1") null true
        (:`EventReceived`
          (bind _returnvalue_4 (`self.GetSpawnLocations`)) ; 获取要生成仆从的点
          (bind _output_get (set `self.SpawnLocations` _returnvalue_4))
          (`KismetArrayLibrary.Array_Shuffle` _output_get) ; 打乱生成的位置数组
          (if (< (`self.SpawnIndex`) (`KismetArrayLibrary.Array_Length` (`self.SpawnLocations`))) :!label _label
            (`NiagaraFunctionLibrary.SpawnSystemAtLocation` "/Game/Assets/Effects/Combat/NS_GroundSummon.NS_GroundSummon" _output)
            (bind _returnvalue_5 (`|SpawnActorFromClass` (`self.GetRandomMinionClass`) (`KismetMathLibrary.MakeTransform` _returnvalue_2 (`KismetMathLibrary.FindLookAtRotation` (`Actor.K2_GetActorLocation` (`self.GetAvatarActorFromActorInfo`)) _returnvalue_2)) "AlwaysSpawn" "MultiplyWithRoot" null null))
            (`Pawn.SpawnDefaultController` _returnvalue_5) ; 手动生成默认控制器
            (add `Actor.OnDestroyed` _returnvalue_5 (delegate `OnDestroyed_Event`)) ; 绑定死亡事件减去已有的仆从数
            (`/Engine/EditorBlueprintResources/StandardMacros.IncrementInt` (`self.SpawnIndex`)
              (:`  `
                (message `CombatInterface.AddMinionCount` (`self.GetAvatarActorFromActorInfo`) 1)
                (`KismetSystemLibrary.Delay` 0.2) ; 间隔生成时间
                (goto _label)))))))))

(event `OnDestroyed_Event`
  (params (DestroyedActor :type "Actor Object Reference"))
  (message `CombatInterface.AddMinionCount` (`self.GetAvatarActorFromActorInfo`) -1))