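; Enemy ranged attack gameplay ability that fires a projectile at the avatar's current facing target.
; On activation it updates facing toward the target through CombatInterface and plays a randomly picked tagged attack montage.
; The montage's gameplay event tag triggers the spawn once, re-reading the target location at that moment for aim.
; The ability ends when the montage completes, is interrupted or is cancelled.
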(event `self.K2_ActivateAbility`
  (bind _returnvalue (`self.GetAvatarActorFromActorInfo`))
  (bind _returnvalue_2 (message `EnemyInterface.GetFacingTarget` _returnvalue))
  (bind _ascombat_interface (cast `CombatInterface` _returnvalue))
  (`CombatInterface.UpdateFacingTarget` _ascombat_interface (`Actor.K2_GetActorLocation` _returnvalue_2))
  (bind _returnvalue_3 (message `EnemyInterface.GetTaggedMontage` (`self.GetAvatarActorFromActorInfo`)))
  (bind _output_get (set `self.AttackMontage` (`self.GetRandomTaggedMontageFromArray` _returnvalue_3)))
  (`AbilityTask_PlayMontageAndWait.CreatePlayMontageAndWaitProxy` "None" (`.CombatMontage` (break `TaggedMontage` _output_get)) 1.0 "None" false
    (:`then`
      (`AbilityTask_WaitGameplayEvent.WaitGameplayEvent` (`.MontageEventTag` (break `TaggedMontage` (`self.AttackMontage`))) null true
        (:`EventReceived`
          (bind _returnvalue_4 (message `EnemyInterface.GetFacingTarget` (`self.GetAvatarActorFromActorInfo`))) ; 获取要面向的目标
          (`self.SpawnProjectile` (`Actor.K2_GetActorLocation` _returnvalue_4)) ; 通过目标位置生成炮弹
        )))
    (:`OnCompleted`
      (`self.K2_EndAbility` :!label _label))
    (:`OnInterrupted`
      (goto _label))
    (:`OnCancelled`
      (goto _label))))