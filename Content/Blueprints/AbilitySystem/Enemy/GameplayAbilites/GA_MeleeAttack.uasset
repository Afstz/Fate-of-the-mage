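; Enemy melee attack gameplay ability that turns the avatar toward its facing target and plays a random tagged attack montage.
; On the montage's tagged gameplay event, it finds living players in a small sphere around the montage's socket and damages those that are not friends.
; If anything was hit, it executes a MeleeImpact gameplay cue at the socket, then ends; it also ends when the montage completes, interrupts or cancels.
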(event `self.K2_ActivateAbility`
  (bind _returnvalue (`self.GetAvatarActorFromActorInfo`))
  (bind _returnvalue_2 (`self.GetAvatarActorFromActorInfo`))
  (bind _attacktaggedmontage (`self.AttackTaggedMontage`))
  (set `self.HitTarget` false)
  (bind _returnvalue_3 (message `EnemyInterface.GetFacingTarget` _returnvalue))
  (bind _ascombat_interface (cast `CombatInterface` _returnvalue))
  (`CombatInterface.UpdateFacingTarget` _ascombat_interface (`Actor.K2_GetActorLocation` _returnvalue_3)) ; 更新要面向的目标
  (bind _returnvalue_4 (message `EnemyInterface.GetTaggedMontage` (`self.GetAvatarActorFromActorInfo`))) ; 获取设置的蒙太奇结构体并随机抽取一个
  (bind _output_get (set `self.AttackTaggedMontage` (`self.GetRandomTaggedMontageFromArray` _returnvalue_4)))
  (`AbilityTask_PlayMontageAndWait.CreatePlayMontageAndWaitProxy` "None" (`.CombatMontage` (break `TaggedMontage` _output_get)) 1.0 "None" false
    (:`then`
      (`AbilityTask_WaitGameplayEvent.WaitGameplayEvent` (`.MontageEventTag` (break `TaggedMontage` _attacktaggedmontage)) null ; 接收指定标签事件
        (:`EventReceived`
          (bind _returnvalue_5 (message `EnemyInterface.GetSocketLocationByStruct` _returnvalue_2 _attacktaggedmontage))
          (bind _output_get_2 (set `self.SocketLocation` _returnvalue_5))
          (bind _outoverlappingactors (`MageAbilitySystemLibrary.GetAlivePlayerInSphereRadius` _returnvalue_2 (`|MakeArray` _returnvalue_2) 40.0 _output_get_2)) ; 查找攻击范围内的击中的角色
          (for _array_element _outoverlappingactors
            (if (`MageAbilitySystemLibrary.IsNotFriend` (`self.GetAvatarActorFromActorInfo`) _array_element)
              (`self.CauseDamage` _array_element)
              (set `self.HitTarget` true)))
          (if (`self.HitTarget`)
            (bind _returnvalue_6 (message `EnemyInterface.GetFacingTarget` (`self.GetAvatarActorFromActorInfo`)))
            (`self.K2_ExecuteGameplayCueWithParams` (struct :`TagName` "GameplayCue.MeleeImpact") (`AbilitySystemBlueprintLibrary.MakeGameplayCueParameters` 0.0 0.0 (struct) (struct) (struct) (`BlueprintGameplayTagLibrary.MakeGameplayTagContainerFromTag` (`.MontageEventTag` (break `TaggedMontage` (`self.AttackTaggedMontage`)))) (struct) (`self.SocketLocation`) (0.0 0.0 0.0) null (`self.GetAvatarActorFromActorInfo`) _returnvalue_6)) ; 执行GameplayCue会自动同步到客户端
          )
          (`self.K2_EndAbility`))))
    (:`OnCompleted`
      (`self.K2_EndAbility` :!label _label))
    (:`OnInterrupted`
      (goto _label))
    (:`OnCancelled`
      (goto _label))))