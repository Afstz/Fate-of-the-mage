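; BP_FlamePillar is a flame pillar actor whose point light flickers randomly.
; On BeginPlay it randomly picks one of two timelines, each scaling the base LightIntensity by its curve value on every update.
; When a timeline finishes it triggers the random pick again, so the flicker loops continuously with a varied pattern and no Event Tick.
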(event `RandomLightIntensity`
  (switch `int` (`KismetMathLibrary.RandomIntegerInRange` 0 1)
    (:`0`
      (`self.LightIntensity_1`))
    (:`1`
      (`self.LightIntensity_2`))))

(event `LightIntensity_1`
  (bind (_direction _intensitymultiply) (`Timeline|LightIntensityTimeline_1` :!via `PlayFromStart`)
    (:`Update`
      (`LightComponent.SetIntensity` (`self.PointLight`) (* _intensitymultiply (`self.LightIntensity`))))
    (:`Finished`
      (`self.RandomLightIntensity`))))

(event `LightIntensity_2`
  (bind (_direction _intensitymultiply) (`Timeline|LightIntensityTimeline_2` :!via `PlayFromStart`)
    (:`Update`
      (`LightComponent.SetIntensity` (`self.PointLight`) (* _intensitymultiply (`self.LightIntensity`))))
    (:`Finished`
      (`self.RandomLightIntensity`))))

(event `self.ReceiveBeginPlay`
  (`self.RandomLightIntensity`))

(fn `UserConstructionScript`)