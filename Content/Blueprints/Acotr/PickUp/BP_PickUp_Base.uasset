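; Base pickup actor Blueprint that handles spawn and removal feedback, using potion sounds.
; On BeginPlay it plays a spawn sound and runs a timeline that offsets its height from CalculatedLocation, scaled by Apex, while animating its scale.
; When the timeline finishes it calls StartMovement, whose logic is not in these graphs.
; Destruction for any reason plays the consume sound at the actor's location.
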(event `self.ReceiveDestroyed`
  (`GameplayStatics.PlaySoundAtLocation` "/Game/Assets/Sounds/Potions/Consume/sfx_Potion_Consume.sfx_Potion_Consume" (`self.K2_GetActorLocation`) (struct) 1.0 1.0 0.0 null null null null))

(event `self.ReceiveBeginPlay`
  (`GameplayStatics.PlaySoundAtLocation` "/Game/Assets/Sounds/Potions/Spawn/sfx_Potion_Spawn.sfx_Potion_Spawn" (`self.K2_GetActorLocation`) (struct) 1.0 1.0 0.0 null null null null)
  (bind (_direction _elevation _scalevalue) (`Timeline|ElevationAndScale`)
    (:`Update`
      (`self.K2_SetActorLocation` (+ (`self.CalculatedLocation`) (`KismetMathLibrary.MakeVector` 0.0 0.0 (* _elevation (`self.Apex`)))))
      (`self.SetActorScale3D` (`KismetMathLibrary.Conv_DoubleToVector` _scalevalue)))
    (:`Finished`
      (`self.StartMovement`))))

(fn `UserConstructionScript`)