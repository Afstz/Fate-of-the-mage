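; Actor implementing FadeInterface that fades its mesh in and out through a timeline-driven "Fade" material parameter.
; The construction script caches the mesh's original materials and builds dynamic instances from FadeMaterialInstances.
; FadeOut applies those instances by slot index and plays the timeline, while Fadein reverses it.
; On finish, a value of 1 restores original materials, and BlockVisibility optionally switches Visibility collision to Block at 1 or Ignore at 0.
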(event `/Game/Blueprints/Acotr/FadeActor/BI_Fade.FadeOut`
  ;[1 1 1] FadeInterface
  (`self.SetMaterialToDynamic`) ; 设置物体为Fade动态材质
  (bind (_direction _fadetrack) (`Timeline|FadeActorTimeline` :!label _label)
    (:`Update`
      (for _array_element (`self.DynamicMaterialInstances`)
        (`MaterialInstanceDynamic.SetScalarParameterValue` _array_element "Fade" _fadetrack)))
    (:`Finished`
      (`self.FadeFinished` _fadetrack))))

(event `/Game/Blueprints/Acotr/FadeActor/BI_Fade.FadeIn`
  ;[1 1 1] FadeInterface
  (goto _label :!via `Reverse`))

(event `self.ReceiveBeginPlay`)

(fn `FadeFinished`
  (params (Value :type "Float (single-precision)"))
  (if (>= Value 1.0)
    (`self.ResetMeshMaterials`) ; 重置物体为初始材质
    (if (`self.bBlockVisibility`)
      (`PrimitiveComponent.SetCollisionResponseToChannel` (`self.Mesh`) "ECC_Visibility" "ECR_Block"))
    (elif (<= Value 0.0)
      (if (`self.bBlockVisibility`)
        (`PrimitiveComponent.SetCollisionResponseToChannel` (`self.Mesh`) "ECC_Visibility" "ECR_Ignore")))))

(fn `ResetMeshMaterials`
  (for (_array_element _array_index) (`self.OriginalMaterials`)
    (`PrimitiveComponent.SetMaterial` (`self.Mesh`) _array_index _array_element)))

(fn `SetMaterialToDynamic`
  (for (_array_element _array_index) (`self.DynamicMaterialInstances`)
    (`PrimitiveComponent.SetMaterial` (`self.Mesh`) _array_index _array_element)))

(fn `UserConstructionScript`
  (`KismetArrayLibrary.Array_Clear` (`self.DynamicMaterialInstances`)) ; 重置
  (set `self.OriginalMaterials` (`MeshComponent.GetMaterials` (`self.Mesh`)))
  (for _array_element (`self.FadeMaterialInstances`)
    (bind _returnvalue (`KismetMaterialLibrary.CreateDynamicMaterialInstance` _array_element))
    (`KismetArrayLibrary.Array_AddUnique` (`self.DynamicMaterialInstances`) _returnvalue)))